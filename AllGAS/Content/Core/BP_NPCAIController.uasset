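; NPC AI controller that keeps its pawn wandering between random reachable navmesh points in a radius around its current location.
; A move-completed binding resets the stored pathfinding status and immediately attempts the next move.
; Tick runs the same check, retrying every frame until a move request succeeds, then idling until that move completes.
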(event Custom|Move%20To%20Random%20Position
  (params (RequestID :type AI%20Request%20ID%20Structure) (Result :type EPathFollowingResult%20Enum :default "Success"))
  (bind _returnvalue (Pawn|GetControlledPawn))
  (bind _returnvalue_2 (Transformation|GetActorLocation _returnvalue))
  (bind (_randomlocation _returnvalue_3) (AI|Navigation|GetRandomReachablePointinRadius _returnvalue_2 1e+03 0 0))
  (Variables|Default|SetPathingFindingStatus "AlreadyAtGoal")
  (if (or false (Utilities|Enum|NotEqual(Enum) (Variables|Default|GetPathingFindingStatus) "RequestSuccessful"))
    (if _returnvalue_3
      (bind _returnvalue_4 (AI|Navigation|MovetoLocation _randomlocation -1.0 false true true true 0))
      (Variables|Default|SetPathingFindingStatus _returnvalue_4))))

(event EventTick
  (params (DeltaSeconds :type Float%20%28single-precision%29))
  (bind _returnvalue (Pawn|GetControlledPawn))
  (bind _returnvalue_2 (Transformation|GetActorLocation _returnvalue))
  (bind (_randomlocation _returnvalue_3) (AI|Navigation|GetRandomReachablePointinRadius _returnvalue_2 1e+03 0 0))
  (if (or false (Utilities|Enum|NotEqual(Enum) (Variables|Default|GetPathingFindingStatus) "RequestSuccessful"))
    (if _returnvalue_3
      (bind _returnvalue_4 (AI|Navigation|MovetoLocation _randomlocation -1.0 false true true true 0))
      (Variables|Default|SetPathingFindingStatus _returnvalue_4))))

(event EventBeginPlay
  (EventDispatchers|BindEventtoReceiveMoveCompleted (delegate Custom|Move%20To%20Random%20Position)))

(fn ConstructionScript)