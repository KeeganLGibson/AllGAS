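; Gameplay ability that extinguishes fires around the avatar by applying GE_PutOutFire to nearby actors.
; An instant WaitTargetData radius query centered on the avatar supplies targets; on valid data it applies the effect to all of them and ends, while cancellation just ends.
; The task's immediate exec output commits the ability for each target tagged Status.fire, without gating the effect on that result.
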(event Ability|EventActivateAbility
  (bind _data (|WaitTargetData :TaskInstanceName "FindFireToPutOut" :ConfirmationType "Instant" :Class "/Script/GameplayAbilities.GameplayAbilityTargetActor_Radius" :Radius 2e+02 :StartLocation (Utilities|Struct|MakeGameplayAbilityTargetingLocationInfo "ActorTransform" "0.000000,0.000000,0.000000|0.000000,0.000000,0.000000|1.000000,1.000000,1.000000" (.avataractor (Ability|GetActorInfo))) :ReticleClass 0 :Filter (Filter|MakeFilterHandle))
    (:then
      (for _array_element (Ability|TargetData|GetActorsfromTargetData _data)
        (if (GameplayTags|HasMatchingGameplayTag (Ability|GetAbilitySystemComponent _array_element) "(TagName=\"status.fire\")")
          (bind _returnvalue (Ability|CommitAbility))
          (if _returnvalue
            _))))
    (:ValidData
      (GameplayEffects|ApplyGameplayEffectToTarget _data "/Game/Core/GameplayAbilities/GE_PutOutFire.GE_PutOutFire_C" 1 1)
      (Ability|EndAbility :!label _label))
    (:Cancelled
      (goto _label))))

(event Ability|EventOnEndAbility
  (params (bWasCancelled :type Boolean)))