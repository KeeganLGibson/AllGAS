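; BP_TargetDummy is a target dummy actor that carries a health bar widget and its own Gameplay Ability System component.
; BeginPlay adds and stores the AbilitySystem component.
; Every Tick reads a float attribute's current and base values from it, and if both are found, passes current divided by base to WBP_HealthBar as health progress.
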(event EventBeginPlay
  (bind _returnvalue (AddComponent|AddAbilitySystemComponent))
  (Variables|Default|SetAbility%20System _returnvalue))

(event Collision|EventActorBeginOverlap
  (params (OtherActor :type Actor%20Object%20Reference)))

(event EventTick
  (params (DeltaSeconds :type Float%20%28single-precision%29))
  (bind _ability_system (Variables|Default|GetAbility%20System))
  (bind (_bsuccessfullyfoundattribute _returnvalue) (Class|AbilitySystemBlueprintLibrary|GetFloatAttributeBasefromAbilitySystemComponent _ability_system "(AttributeName=\"Health\",Attribute=/Script/AllGAS.AGBaseAttributeSet:Health,AttributeOwner=None)"))
  (bind (_bsuccessfullyfoundattribute_2 _returnvalue_2) (Ability|Attribute|GetFloatAttributefromAbilitySystemComponent _ability_system "(AttributeName=\"Health\",Attribute=/Script/AllGAS.AGBaseAttributeSet:Health,AttributeOwner=None)"))
  (if (and _bsuccessfullyfoundattribute _bsuccessfullyfoundattribute_2)
    (bind _aswbp_health_bar (Utilities|Casting|CastToWBP_HealthBar (UserInterface|GetWidget (Variables|Default|GetHealth%20Bar))))
    (Default|SetHealthProgress _aswbp_health_bar (/ _returnvalue_2 _returnvalue))))

(fn ConstructionScript)